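; ViewerBP is the player-side viewer for MSP and IMF data windows, owning the main menu and cursor info widgets.
; BeginPlay creates both widgets, sets up mouse and camera, and draws the color wheel to a render target after a delay.
; Tick syncs the title to the selected channel's wavelength and shows hover time, value and zenith angle.
; Events hide panels during screenshot export and link the IMF window to its legend.
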(event `self.ReceiveBeginPlay`
  (bind _returnvalue (`|CreateWidget` "/Game/Blueprints/Widgets/MainMenuWidget.MainMenuWidget_C"))
  (set `self.MenuWidget` _returnvalue)
  (set `self.MainMenuRef` _returnvalue)
  (`UserWidget.AddToViewport` _returnvalue 0)
  (`GameplayStatics.SetViewportMouseCaptureMode` "CapturePermanently_IncludingInitialMouseDown")
  (set `PlayerController.bShowMouseCursor` true (`GameplayStatics.GetPlayerController` 0))
  (set `self.PrevChannel` -1)
  (bind _returnvalue_2 (`|CreateWidget` "/Game/Blueprints/Widgets/MouseInfoWidget.MouseInfoWidget_C"))
  (set `self.CursorInfoWidget` _returnvalue_2)
  (`UserWidget.AddToViewport` _returnvalue_2 1)
  (set `CameraComponent.AspectRatio` 1.0 (`self.Camera`))
  (`KismetSystemLibrary.Delay` 1.0)
  (`KismetRenderingLibrary.DrawMaterialToRenderTarget` "/Game/Textures/ColorWheelRenderTarget.ColorWheelRenderTarget" "/Game/Materials/ColorWheelMaterial_Inst.ColorWheelMaterial_Inst"))

(event `self.ReceiveTick`
  (params (DeltaSeconds :type "Float (single-precision)"))
  (bind _returnvalue (`GameplayStatics.GetPlayerController` 0))
  (bind _cursorinfowidget (`self.CursorInfoWidget`))
  (bind _mspwindows (break `WindowManager` (`self.windows`)))
  (if (not (`PlayerController.bShowMouseCursor` _returnvalue))
    (set `PlayerController.bShowMouseCursor` true _returnvalue))
  (if (> (`KismetArrayLibrary.Array_Length` _mspwindows) 0)
    (bind _asmain_menu_widget (cast `/Game/Blueprints/Widgets/MainMenuWidget` (`self.MenuWidget`)))
    (bind _returnvalue_2 (`KismetMathLibrary.FFloor` (`SpinBox.GetValue` (`/Game/Blueprints/Widgets/MainMenuWidget.ChannelBox` _asmain_menu_widget))))
    (if (!= (`self.PrevChannel`) _returnvalue_2)
      (set `self.PrevChannel` _returnvalue_2)
      (`/Game/Blueprints/Widgets/MainMenuWidget.SetTitleText` _asmain_menu_widget (`KismetStringLibrary.Conv_DoubleToString` (`|GetArrayItem` (`MSPWindow.mspWavelengths` (`|GetArrayItem` _mspwindows)) _returnvalue_2)))
      (bind _returnvalue_3 (`self.getWindows`)))
    (bind _mspwindows_2 (break `WindowManager` _returnvalue_3))
    (bind _output (`|GetArrayItem` _mspwindows_2))
    (if (`KismetSystemLibrary.IsValid` _output)
      (if (> (`KismetArrayLibrary.Array_Length` _mspwindows_2) 0)
        (`/Game/Blueprints/Widgets/MouseInfoWidget.SetTimeText` _cursorinfowidget (`/Game/Blueprints/Widgets/MainMenuWidget.ConvertSecondsToTimeStamp` _asmain_menu_widget (`MSPWindow.mspHoverTime` _output)))
        (`/Game/Blueprints/Widgets/MouseInfoWidget.SetValueText` _cursorinfowidget (`KismetStringLibrary.Conv_DoubleToString` (`MSPWindow.mspHoverValue` _output)))
        (bind (_mouseuv_x _mouseuv_y) (`KismetMathLibrary.BreakVector2D` (`MSPWindow.mouseUV` _output)))
        (set `TextBlock.Text` (`KismetTextLibrary.Conv_StringToText` (`KismetStringLibrary.Concat_StrStr` "Zenith: " (`KismetTextLibrary.Conv_TextToString` (`KismetTextLibrary.Conv_IntToText` (`KismetMathLibrary.FFloor` (* (- 1.0 _mouseuv_y) 181.0)))) "°")) (`/Game/Blueprints/Widgets/MouseInfoWidget.AngleText` (`self.CursorInfoWidget`)))
        (else
          (`KismetSystemLibrary.PrintString` "Apparently there arent any msp windows" true true (struct :`G` 0.66 :`B` 1.0 :`A` 1.0) 0.0))))))

(event `self.OnBeforeExportScreenshot`
  (bind _mainmenuref (`self.MainMenuRef`))
  (bind _returnvalue (`KismetSystemLibrary.IsValid` _mainmenuref))
  (if _returnvalue
    (`Widget.SetVisibility` (`/Game/Blueprints/Widgets/MainMenuWidget.MSPPanel` _mainmenuref) "Collapsed"))
  (bind _asimfwindow_bp (cast `/Game/Blueprints/Windows/IMFWindowBP` (`self.imfWindow`)))
  (if (`KismetSystemLibrary.IsValid` _asimfwindow_bp)
    (if (`KismetSystemLibrary.IsValid` (`/Game/Blueprints/Windows/IMFWindowBP.ArcTanManager` _asimfwindow_bp))
      (bind _imfmanager (`/Game/Blueprints/Windows/IMFWindowBP.IMFManager` _asimfwindow_bp))
      (if (`KismetSystemLibrary.IsValid` _imfmanager)
        (if _returnvalue
          (`Widget.SetVisibility` _imfmanager "Collapsed")
          (`Widget.SetVisibility` (`/Game/Blueprints/Windows/IMFWindowBP.ArcTanManager` _asimfwindow_bp) "Collapsed"))))))

(event `self.OnAfterExportScreenshot`
  (bind _mainmenuref (`self.MainMenuRef`))
  (bind _returnvalue (`KismetSystemLibrary.IsValid` _mainmenuref))
  (if _returnvalue
    (`Widget.SetVisibility` (`/Game/Blueprints/Widgets/MainMenuWidget.MSPPanel` _mainmenuref) "Visible"))
  (bind _asimfwindow_bp (cast `/Game/Blueprints/Windows/IMFWindowBP` (`self.imfWindow`)))
  (if (`KismetSystemLibrary.IsValid` _asimfwindow_bp)
    (bind _imfmanager (`/Game/Blueprints/Windows/IMFWindowBP.IMFManager` _asimfwindow_bp))
    (if (`KismetSystemLibrary.IsValid` _imfmanager)
      (if (`KismetSystemLibrary.IsValid` (`/Game/Blueprints/Windows/IMFWindowBP.ArcTanManager` _asimfwindow_bp))
        (if _returnvalue
          (`Widget.SetVisibility` _imfmanager "Visible")
          (`Widget.SetVisibility` (`/Game/Blueprints/Windows/IMFWindowBP.ArcTanManager` _asimfwindow_bp) "Visible"))))))

(event `self.OnIMFWindowSpawned`
  (bind _imfwindow (`self.imfWindow`))
  (bind _asimfwindow_bp (cast `/Game/Blueprints/Windows/IMFWindowBP` _imfwindow))
  (set `/Game/Blueprints/Widgets/IMFLegendWidget.WindowRef` _asimfwindow_bp (`/Game/Blueprints/Widgets/MainMenuWidget.IMFLegendWidget` (`self.MainMenuRef`)))
  (add `IMFWindow.OnIMFLegendChanged` _imfwindow (delegate `OnLegendUpdated`)))

(event `OnLegendUpdated`
  (`/Game/Blueprints/Widgets/IMFLegendWidget.RebuildLegend` (`/Game/Blueprints/Widgets/MainMenuWidget.IMFLegendWidget` (`self.MainMenuRef`))))

(fn `UserConstructionScript`)